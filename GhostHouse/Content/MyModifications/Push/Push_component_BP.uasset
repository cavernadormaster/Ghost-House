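; Character component that lets its owner push an object along the owner's forward direction.
; BeginPush attaches the character to the pushable, plane-constrains movement by its right vector, stops orient-to-movement and enables tick; EndPush reverses this.
; While active, Tick moves the pushable with a swept offset at PushSpeed, carrying the attached character and printing collision debug.
; Helpers report whether a push is active and the pushable's top height above the character's feet.
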(event EventBeginPlay
  (Components|Tick|SetComponentTickEnabled false))

(event EventTick
  (params (DeltaSeconds :type Float%20%28single-precision%29))
  (bind _currentpushable (Variables|Default|GetcurrentPushable)
    (:then
      (bind _sweephitresult (Transformation|AddActorWorldOffset _currentpushable (* (Transformation|GetActorForwardVector (Components|GetOwner)) (* DeltaSeconds (Variables|Default|GetPushSpeed))) true))
      (Development|PrintString (Utilities|String|Append "Collided with:" (Utilities|GetDisplayName (.HitActor (Collision|BreakHitResult _sweephitresult)))) true true (select (.bBlockingHit (Collision|BreakHitResult _sweephitresult)) "(R=0.000000,G=1.979682,B=2.000000,A=1.000000)" "(R=1.000000,G=0.000000,B=0.000000,A=1.000000)") 0.0))
    (:else)))

(fn BeginPush
  (params (Pushable :type Push%20BP%20Object%20Reference))
  (if (not (Utilities|IsValid (Variables|Default|GetcurrentPushable)))
    (bind _ascharacter (Utilities|Casting|CastToCharacter (Components|GetOwner)))
    (LocalVariables|SetOwnerCahracte _ascharacter)
    (bind _output_get (Variables|Default|SetcurrentPushable Pushable))
    (Transformation|AttachActorToActor (LocalVariables|GetOwnerCahracte) _output_get "None" "KeepWorld" "KeepWorld" "KeepWorld" true)
    (Class|MovementComponent|SetPlaneConstraintEnabled (Variables|/Script/Engine.Character|GetCharacterMovement (LocalVariables|GetOwnerCahracte)) true)
    (Class|MovementComponent|SetPlaneConstraintNormal (Variables|/Script/Engine.Character|GetCharacterMovement (LocalVariables|GetOwnerCahracte)) (Transformation|GetActorRightVector (LocalVariables|GetOwnerCahracte)))
    (Variables|/Script/Engine.CharacterMovementComponent|SetbOrientRotationToMovement (Variables|/Script/Engine.Character|GetCharacterMovement (LocalVariables|GetOwnerCahracte)) false)
    (Components|Tick|SetComponentTickEnabled true)))

(fn EndPush
  (Variables|Default|GetcurrentPushable
    (:then
      (Variables|Default|SetcurrentPushable 0)
      (bind _ascharacter (Utilities|Casting|CastToCharacter (Components|GetOwner)))
      (bind _output_get (LocalVariables|SetOwningCharacter _ascharacter))
      (Transformation|DetachFromActor _output_get "KeepWorld" "KeepWorld" "KeepWorld")
      (Class|MovementComponent|SetPlaneConstraintEnabled (Variables|/Script/Engine.Character|GetCharacterMovement (LocalVariables|GetOwningCharacter)) false)
      (Variables|/Script/Engine.CharacterMovementComponent|SetbOrientRotationToMovement (Variables|/Script/Engine.Character|GetCharacterMovement (LocalVariables|GetOwningCharacter)) true)
      (Components|Tick|SetComponentTickEnabled false))
    (:else)))

(fn IsPushingObject
  (return (Utilities|IsValid (Variables|Default|GetcurrentPushable))))

(fn GetPushableHeight
  (Utilities|FlowControl|Sequence
    (:then_0
      (bind _currentpushable (Variables|Default|GetcurrentPushable)
        (:then
          (LocalVariables|Settop%20of%20object (+ (- (.z (.Max (Components|StaticMesh|GetLocalBounds (Variables|/Game/MyModifications/Push/Push_BP.Push_BP_C|GetStaticMesh _currentpushable)))) (.z (.Min (Components|StaticMesh|GetLocalBounds (Variables|/Game/MyModifications/Push/Push_BP.Push_BP_C|GetStaticMesh _currentpushable))))) (.z (Transformation|GetActorLocation (Variables|Default|GetcurrentPushable)))))
          (bind _ascharacter (Utilities|Casting|CastToCharacter (Components|GetOwner)))
          (LocalVariables|SetFeet%20of%20Character (- (.z (Transformation|GetActorLocation _ascharacter)) (Components|Capsule|GetScaledCapsuleHalfHeight (Variables|/Script/Engine.Character|GetCapsuleComponent _ascharacter))))
          (return (- (LocalVariables|Gettop%20of%20object) (LocalVariables|GetFeet%20of%20Character))))
        (:else)))
    (:then_1
      (return 0.0))))