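; Pushable object actor that, on interact, snaps a character to the nearest push point and starts a push through its Push_component_BP.
; Editable push transforms are shown as arrow components by the construction script.
; It picks the closest transform within the component's push range, then validates standing room, walkable floor and line of sight with capsule and line traces before teleporting.
; Failures print a red reason, and traces draw debug shapes.
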(event EventBeginPlay)

(event Collision|EventActorBeginOverlap
  (params (OtherActor :type Actor%20Object%20Reference)))

(event EventTick
  (params (DeltaSeconds :type Float%20%28single-precision%29)))

(event EventInterect
  (params (Human%20 :type Human%20Object%20Reference))
  (CallFunction|HandleInteraction Human%20))

(fn ConstructionScript
  (for _array_element (Variables|Default|GetpushTranforms)
    (AddComponent|AddArrowComponent false _array_element)))

(fn HandleInteraction
  (params (chracter :type Character%20Object%20Reference))
  (bind _capsulecomponent (Variables|/Script/Engine.Character|GetCapsuleComponent chracter))
  (Utilities|IsValid chracter
    (:Is%20Valid
      (bind _output_get (LocalVariables|SetPushCOmponent (Actor|GetComponentbyClass chracter "/Game/MyModifications/Push/Push_component_BP.Push_component_BP_C")))
      (Utilities|IsValid _output_get
        (:Is%20Valid
          (bind _best_index (CallFunction|FindClosesPushTransformIndex (Math|Conversions|ToVector2D(Vector) (Transformation|GetActorLocation chracter)) (Variables|/Game/MyModifications/Push/Push_component_BP.Push_component_BP_C|GetPushRange (LocalVariables|GetPushCOmponent))))
          (if (>= _best_index 0)
            (bind _output_get_2 (LocalVariables|SetCharacterNewTranform (Math|Transform|MakeTransform (+ (.location (Math|Transform|ComposeTransforms (Utilities|Array|Get(acopy) (Variables|Default|GetpushTranforms) _best_index) (Transformation|GetActorTransform))) (Math|Vector|MakeVector 0.0 0.0 (Components|Capsule|GetScaledCapsuleHalfHeight (Variables|/Script/Engine.Character|GetCapsuleComponent chracter)))) (.rotation (Math|Transform|ComposeTransforms (Utilities|Array|Get(acopy) (Variables|Default|GetpushTranforms) _best_index) (Transformation|GetActorTransform))) (.scale (Math|Transform|ComposeTransforms (Utilities|Array|Get(acopy) (Variables|Default|GetpushTranforms) _best_index) (Transformation|GetActorTransform))))))
            (Rendering|Debug|DrawDebugSphere (.location _output_get_2) 2e+01 12 "(R=1.000000,G=0.000000,B=0.020607,A=1.000000)" 2.0)
            (bind _outhit (Collision|CapsuleTraceByChannel (+ (.location (LocalVariables|GetCharacterNewTranform)) "0, 0,70.000000") (- (.location (LocalVariables|GetCharacterNewTranform)) "0, 0,100.000000") (Components|Capsule|GetScaledCapsuleRadius _capsulecomponent) (Components|Capsule|GetScaledCapsuleHalfHeight _capsulecomponent) "TraceTypeQuery1" false 0 "ForDuration" true "(R=1.000000,G=0.000000,B=0.000000,A=1.000000)" "(R=0.000000,G=1.000000,B=0.000000,A=1.000000)" 2.0))
            (if (not (.bInitialOverlap (Collision|BreakHitResult _outhit)))
              (if (< (Class|CharacterMovementComponent|GetWalkableFloorZ (Variables|/Script/Engine.Character|GetCharacterMovement chracter)) (.Z (Math|Vector|BreakVector (.ImpactNormal (Collision|BreakHitResult _outhit)))))
                (bind _returnvalue (Collision|LineTraceByChannel (Transformation|GetActorLocation) (.location (LocalVariables|GetCharacterNewTranform)) "TraceTypeQuery1" false (Utilities|Array|MakeArray chracter) "ForDuration" true "(R=1.000000,G=0.000000,B=0.000000,A=1.000000)" "(R=0.000000,G=1.000000,B=0.000000,A=1.000000)" 2.0))
                (if (not _returnvalue)
                  (Transformation|SetActorTransform chracter (LocalVariables|GetCharacterNewTranform) false true)
                  (Default|BeginPush (LocalVariables|GetPushCOmponent) self)
                  (else
                    (Utilities|PushFailedInfo "WALL IN BETWEEN PLAYER AND OBJECT")))
                (else
                  (Utilities|PushFailedInfo "FLOOR NOT WALKABLE")))
              (else
                (Utilities|PushFailedInfo "NO ROOM TO STAND")))
            (else
              (Utilities|PushFailedInfo "NO PUSH TRANSFORM FOUND "))))
        (:Is%20Not%20Valid
          (Utilities|PushFailedInfo "chracter doent have push component"))))
    (:Is%20Not%20Valid
      (Utilities|PushFailedInfo "chracter is invalid"))))

(fn FindClosesPushTransformIndex
  (params (character%20location :type Vector%202D%20Structure) (Push%20Range :type Float%20%28single-precision%29))
  (for (_array_element _array_index) (Variables|Default|GetpushTranforms)
    (LocalVariables|SetcurentTransformIndex _array_index)
    (bind _output_get (LocalVariables|SetCurrentDistanceSq (Class|KismetMathLibrary|DistanceSquared2D (Math|Conversions|ToVector2D(Vector) (Math|Transform|TransformLocation (Transformation|GetActorTransform) (.location _array_element))) character%20location)))
    (if (< _output_get (Math|Float|Square Push%20Range))
      (if (or (< (LocalVariables|GetCurrentDistanceSq) (LocalVariables|GetCloastestDistanceSq)) (< (LocalVariables|GetClosestTranformIndex) 0))
        (LocalVariables|SetClosestTranformIndex (LocalVariables|GetcurentTransformIndex))
        (LocalVariables|SetCloastestDistanceSq (LocalVariables|GetCurrentDistanceSq)))))
  (return (LocalVariables|GetClosestTranformIndex)))